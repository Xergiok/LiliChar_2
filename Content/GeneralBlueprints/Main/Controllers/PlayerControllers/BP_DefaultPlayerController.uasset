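; Default player controller that handles pause, interaction, physics grabbing, camera FOV and a distortion effect.
; A forward sphere trace from the camera manager sends a main-action message to hit actors or feeds light simulating components to the character's PhysicsHandle.
; Distortion pairs an FOV-oscillation camera shake with an additive post-process material, toggled by a numpad key.
; The held-object target update is disconnected, and Tick is empty.
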(event `self.ReceiveTick`
  (params (DeltaSeconds :type "Float (single-precision)")))

(event `self.ReceiveBeginPlay`
  ;[1 0.4676 0] Event BeginPlay
  (bind _output_get (set `self.PlayerCharacter` (`/Game/GeneralBlueprints/Main/MacroLibrary/MCL_Actor_MacroLibrary.MCL_Get_DPlayerCharacter`)))
  (set `self.CurrentCamera` (`/Game/GeneralBlueprints/Main/Characters/Player/BP_HumanCharacter.FP Camera` _output_get))
  (`self.Set_ClampedFOV` (`self.Base_FOV`)))

(event `InputAction|Pause Game` :paused true
  (params (Key :type "Key Structure"))
  ;[0 0.6682 1] Pause
  (:`Pressed`
    (bind _isa (`/Engine/EditorBlueprintResources/StandardMacros.FlipFlop`)
      (:`A`
        _)
      (:`B`
        _))
    (`GameplayStatics.SetGamePaused` _isa)))

(event `InputAction|Main Action`
  (params (Key :type "Key Structure"))
  ;[0 0.6682 1] Line Trace
  (:`Pressed`
    (bind _last_hit_actor (`self.Simple SphereTrace`))
    (message `/Game/GeneralBlueprints/Main/Interfaces/BPI_Interaction.Main_Action` _last_hit_actor)))

(event `InputAction|Side Action`
  (params (Key :type "Key Structure"))
  ;[0 0.6682 1] Line Trace
  (:`Pressed`
    (bind (_last_hit_actor _last_hit_actorcomp) (`self.Simple SphereTrace`))
    (`self.Grab Component` _last_hit_actorcomp))
  (:`Released`
    (`self.Drop Component`)))

(event `Start_DistortionEffect`
  ;[1 1 1] Distortion
  (`self.ClientStartCameraShake` "/Game/GeneralBlueprints/Miscellanious/CameraShake/FOV_Ocillation.FOV_Ocillation_C" (`self.FOV_Osc_Scale`))
  (`self.Set Additive Post Proc Mat` 1.0 (make `WeightedBlendable` 1.0 "/Game/Materials/Mat_Distortion.Mat_Distortion")))

(event `Key|NumPadFive`
  (params (Key :type "Key Structure"))
  ;[1 0 0.01005] Comment
  (:`Pressed`
    (`/Engine/EditorBlueprintResources/StandardMacros.FlipFlop`
      (:`A`
        (`self.Start_DistortionEffect`))
      (:`B`
        (`self.Stop_DistortionEffect`)))))

(event `Stop_DistortionEffect`
  ;[1 1 1] Distortion
  (`self.ClientStopCameraShake` "/Game/GeneralBlueprints/Miscellanious/CameraShake/FOV_Ocillation.FOV_Ocillation_C" false)
  (`self.Set Additive Post Proc Mat` 1.0))

(fn `Drop Component`
  (`PhysicsHandleComponent.ReleaseComponent` (`/Game/GeneralBlueprints/Main/Characters/Player/BP_HumanCharacter.PhysicsHandle` (`/Game/GeneralBlueprints/Main/MacroLibrary/MCL_Actor_MacroLibrary.MCL_Get_DPlayerCharacter`)))
  (set `self.HoldComponent` false))

(fn `Grab Component`
  (params (Component :type "PrimitiveComponent Object Reference"))
  (`/Engine/EditorBlueprintResources/StandardMacros.IsValid` Component
    (:`Is Valid`
      (if (and (`SceneComponent.IsSimulatingPhysics` Component "None") (< (`PrimitiveComponent.GetMass` Component) 100.0))
        (if (not (`self.HoldComponent`))
          (set `self.HoldComponent` true)
          (`PhysicsHandleComponent.GrabComponentAtLocation` (`/Game/GeneralBlueprints/Main/Characters/Player/BP_HumanCharacter.PhysicsHandle` (`/Game/GeneralBlueprints/Main/MacroLibrary/MCL_Actor_MacroLibrary.MCL_Get_DPlayerCharacter`)) Component "None" (`SceneComponent.K2_GetComponentLocation` Component)))))))

(fn `Set Additive Post Proc Mat`
  (params (BlendWeight :type "Float (double-precision)") (PostProc_Mat :type "WeightedBlendable Structure"))
  (bind _postprocess_additive (`self.PostProcess_Additive`))
  (set `PostProcessComponent.BlendWeight` BlendWeight _postprocess_additive)
  (set `PostProcessComponent.Settings` (make `PostProcessSettings` :`WeightedBlendables` (make `WeightedBlendables` (`|MakeArray` PostProc_Mat))) _postprocess_additive))

(fn `Set_ClampedFOV`
  (params (Value :type "Float (double-precision)"))
  (bind _currentcamera (`self.CurrentCamera`)
    (:`then`
      (`CameraComponent.SetFieldOfView` _currentcamera (`KismetMathLibrary.FClamp` Value 5.0 170.0)))
    (:`else`)))

(fn `Set_DesiredControl_Rotation`
  (params (Rot :type "Rotator Structure") (InterpSpeed :type "Float (double-precision)"))
  (`self.SetControlRotation` (`KismetMathLibrary.RInterpTo` (`self.GetControlRotation`) Rot (`GameplayStatics.GetWorldDeltaSeconds`) InterpSpeed)))

(fn `Simple SphereTrace`
  (returns (Last_Hit_Actor :type "Actor Object Reference") (Last_Hit_ActorComp :type "PrimitiveComponent Object Reference"))
  (locals (Trace :type Boolean) (LineTrace_Length :type "Float (double-precision)" :default 100.0) (SphereRadius :type "Float (double-precision)" :default 2.0))
  (bind _rootcomponent (`Actor.RootComponent` (`self.PlayerCameraManager`)))
  (bind _returnvalue (`SceneComponent.K2_GetComponentLocation` _rootcomponent))
  (bind (_outhit _returnvalue_2) (`KismetSystemLibrary.SphereTraceSingleForObjects` :`Start` _returnvalue :`End` (+ _returnvalue (* (`SceneComponent.GetForwardVector` _rootcomponent) (`local.LineTrace_Length`))) :`Radius` (`local.SphereRadius`) :`ObjectTypes` (`|MakeArray` "ObjectTypeQuery1" "ObjectTypeQuery2" "ObjectTypeQuery4" :!type "EObjectTypeQuery Enum") :`DrawDebugType` "ForDuration"))
  (if _returnvalue_2
    (bind (_bblockinghit _binitialoverlap _time _distance _location _impactpoint _normal _impactnormal _physmat _hitactor _hitcomponent) (`GameplayStatics.BreakHitResult` _outhit))
    (set `local.Trace` _bblockinghit)
    (`/Engine/EditorBlueprintResources/StandardMacros.IsValid` _hitactor
      (:`Is Valid`
        (`/Engine/EditorBlueprintResources/StandardMacros.IsValid` _hitcomponent
          (:`Is Valid`
            (return _hitactor _hitcomponent)))))))

(fn `UserConstructionScript`
  (set `self.GameInstance` (`/Game/GeneralBlueprints/Main/MacroLibrary/MCL_Actor_MacroLibrary.MCL_Get_DGameInstance`))
  (set `self.GameMode` (`/Game/GeneralBlueprints/Main/MacroLibrary/MCL_Actor_MacroLibrary.MCL_Get_DGameMode`)))