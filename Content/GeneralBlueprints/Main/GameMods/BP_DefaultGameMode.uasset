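; Default game mode that caches references to the human player character and its animation instance on BeginPlay.
; It then creates a test HUD widget, adds it to the viewport and hands it a reference to itself.
; A separate update function copies the crouch, walk and sprint hold input settings from its settings struct onto the player character.
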(event `self.ReceiveBeginPlay`
  (`self.Add_Reference_to_Player`)
  (`self.Add_Reference_to_PlayerAnimation`)
  (`self.Add_Test_Widget`))

(fn `Add_Reference_to_Player`
  (bind _asbp_human_character (cast `/Game/GeneralBlueprints/Main/Characters/Player/BP_HumanCharacter` (`GameplayStatics.GetPlayerCharacter` 0)))
  (set `self.PlayerCharacter` _asbp_human_character))

(fn `Add_Reference_to_PlayerAnimation`
  (bind _playercharacter (`self.PlayerCharacter`)
    (:`then`
      (bind _asabp_general_human_character (cast `/Game/AnimAssets/Characters/TestChar/Animations/TestCharAnims/CharAnimationInstances/ABP_General_HumanCharacter` (`SkeletalMeshComponent.GetAnimInstance` (`Character.Mesh` _playercharacter))))
      (set `self.Player Animation` _asabp_general_human_character))
    (:`else`)))

(fn `Add_Test_Widget`
  (`self.PlayerCharacter`
    (:`then`
      (bind _returnvalue (`|CreateWidget` "/Game/GeneralBlueprints/debugHUD/UMG_UI_TestHUD.UMG_UI_TestHUD_C"))
      (set `self.TestWidget` _returnvalue)
      (`UserWidget.AddToViewport` _returnvalue 0)
      (set `/Game/GeneralBlueprints/debugHUD/UMG_UI_TestHUD.GameMode` self _returnvalue))
    (:`else`)))

(fn `Update_PlayerSettings`
  (`|ExecutionSequence`
    (:`then_0`
      (set `/Game/GeneralBlueprints/Main/Characters/Player/BP_HumanCharacter.crouch_settings_hold` (`.InputSettings_Crouch_Hold_3_59ED9E7F4470D4E8892935B6FA4A0FC3` (break `/Game/GeneralBlueprints/Miscellanious/KeySettings/ST_Player_KeypressSettings` (`self.ST_Input_Settings`))) (`self.PlayerCharacter`)))
    (:`then_1`
      (set `/Game/GeneralBlueprints/Main/Characters/Player/BP_HumanCharacter.walk_settings_hold` (`.InputSettings_Walk_Hold_4_C5E9AA7142969297911FE49B5829AC61` (break `/Game/GeneralBlueprints/Miscellanious/KeySettings/ST_Player_KeypressSettings` (`self.ST_Input_Settings`))) (`self.PlayerCharacter`)))
    (:`then_2`
      (set `/Game/GeneralBlueprints/Main/Characters/Player/BP_HumanCharacter.sprint_settings_hold` (`.InputSettings_Sprint_Hold_5_26A9FF3E489CB4926C0588AF4987C67E` (break `/Game/GeneralBlueprints/Miscellanious/KeySettings/ST_Player_KeypressSettings` (`self.ST_Input_Settings`))) (`self.PlayerCharacter`)))))

(fn `UserConstructionScript`)